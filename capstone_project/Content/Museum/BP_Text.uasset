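; BP_Text is a museum text actor with Title and Description components that appear only while a player is in.
; Both start hidden on BeginPlay, and the PlayerIn and PlayerOut events show and hide them; nothing in this graph calls those events.
; Two timelines that would move each component along Z are disconnected and never run.
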(event Custom|PlayerIn
  (Rendering|SetVisibility (Variables|Default|GetTitle) true false)
  (Rendering|SetVisibility (Variables|Default|GetDescription) true false))

(event Custom|PlayerOut
  (Rendering|SetVisibility (Variables|Default|GetTitle) false false)
  (Rendering|SetVisibility (Variables|Default|GetDescription) false false))

(event EventBeginPlay
  (Rendering|SetVisibility (Variables|Default|GetTitle) false false)
  (Rendering|SetVisibility (Variables|Default|GetDescription) false false))

(event Collision|EventActorBeginOverlap
  (params (OtherActor :type Actor%20Object%20Reference)))

(event EventTick
  (params (DeltaSeconds :type Float%20%28single-precision%29)))

(fn ConstructionScript)